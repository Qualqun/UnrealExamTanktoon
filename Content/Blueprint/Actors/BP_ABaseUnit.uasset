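; Base unit actor that handles automatic projectile fire and health.
; StartShoot runs a looping fire-rate timer, with a negative initial delay for an immediate first shot, until StopShoot clears it.
; A CanShoot cooldown timer prevents re-trigger spam.
; Shoot spawns BP_AProjectile at MuzzlePoint, passing owner and damage, while TakeDamage simply subtracts from Hp.
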(event `ActiveShoot`
  (set `self.CanShoot` true))

(event `Shoot`
  (bind _returnvalue (`|SpawnActorFromClass` "/Game/Blueprint/Actors/BP_AProjectile.BP_AProjectile_C" (`SceneComponent.K2_GetComponentToWorld` (`self.MuzzlePoint`)) "Undefined" "MultiplyWithRoot" null null))
  (`Bullet.SetOwnerActor` _returnvalue self)
  (`Bullet.SetBulletDamage` _returnvalue (`self.Damage`)))

(event `self.TakeDamage`
  (params (DamageAmount :type Integer))
  (set `self.Hp` (- (`self.Hp`) DamageAmount)))

(fn `StartShoot`
  (bind _firerate (`self.FireRate`))
  (if (`KismetSystemLibrary.K2_IsValidTimerHandle` (`self.TimerShoot`))
    _
    (elif (`self.CanShoot`)
      (bind _returnvalue (`KismetSystemLibrary.K2_SetTimerDelegate` (`|CreateDelegate` :!event `Shoot`) _firerate true false (* _firerate -1.0)))
      (set `self.TimerShoot` _returnvalue)
      (set `self.CanShoot` false)
      (`KismetSystemLibrary.K2_SetTimerDelegate` (`|CreateDelegate` :!event `ActiveShoot`) (`self.FireRate`)) ; Useful for preventing spam
    )))

(fn `StopShoot`
  (`KismetSystemLibrary.K2_ClearAndInvalidateTimerHandle` (`self.TimerShoot`)))

(fn `UserConstructionScript`)