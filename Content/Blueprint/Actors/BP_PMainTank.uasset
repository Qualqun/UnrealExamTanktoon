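; BP_PMainTank is the player's tank, moved and rotated by Enhanced Input, with shoot input calling StartShoot and StopShoot.
; Input is disabled on BeginPlay, to be enabled by the game manager, per the author's note.
; Each tick the turret yaws toward the point under the cursor.
; On destruction it spawns a camera actor at its camera's transform as view target and notifies GM_TankToon of player death.
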(event `self.ReceiveBeginPlay`
  (bind _returnvalue (`GameplayStatics.GetPlayerController` 0))
  ;[1 1 1] Set input, they gona be enabled on game manager
  (`parent.ReceiveBeginPlay`)
  (`self.DisableInput` _returnvalue)
  (`EnhancedInputSubsystemInterface.AddMappingContext` (pcsubsystem `EnhancedInputLocalPlayerSubsystem` _returnvalue) "/Game/Blueprint/Inputs/InputMappingContext.InputMappingContext" 0 (struct)))

(event `EnhancedInput|/Game/Blueprint/Inputs/Inputs/ForwardBackward`
  (params (ActionValue :type "Float (double-precision)") (ElapsedSeconds :type "Float (double-precision)") (TriggeredSeconds :type "Float (double-precision)") (InputAction :type "InputAction Object Reference" :default "/Game/Blueprint/Inputs/Inputs/ForwardBackward.ForwardBackward"))
  (:`Triggered`
    (`self.K2_AddActorWorldOffset` (* ActionValue (`SceneComponent.GetForwardVector` (`self.BaseUnit`)) (`self.Speed`)) true)))

(event `EnhancedInput|/Game/Blueprint/Inputs/Inputs/Rotate`
  (params (ActionValue :type "Float (double-precision)") (ElapsedSeconds :type "Float (double-precision)") (TriggeredSeconds :type "Float (double-precision)") (InputAction :type "InputAction Object Reference" :default "/Game/Blueprint/Inputs/Inputs/Rotate.Rotate"))
  (:`Triggered`
    (`SceneComponent.K2_AddWorldRotation` (`self.BaseUnit`) (`KismetMathLibrary.MakeRotator` 0.0 0.0 (* ActionValue (`self.SpeedRotate`))) false false)))

(event `self.ReceiveTick`
  (params (DeltaSeconds :type "Float (single-precision)"))
  (bind (_returnvalue_roll _returnvalue_pitch _returnvalue_yaw) (`KismetMathLibrary.BreakRotator` (`KismetMathLibrary.FindLookAtRotation` (`SceneComponent.K2_GetComponentLocation` (`self.TankTurret`)) (`.Location` (`GameplayStatics.BreakHitResult` (`PlayerController.GetHitResultUnderCursorByChannel` (`GameplayStatics.GetPlayerController` 0) "TraceTypeQuery1" true))))))
  (`/Engine/EditorBlueprintResources/StandardMacros.IsValid` (`self.MuzzlePoint`)
    (:`Is Valid`
      (`SceneComponent.K2_SetWorldRotation` (`self.TankTurret`) (`KismetMathLibrary.MakeRotator` 0.0 0.0 _returnvalue_yaw) false false))))

(event `self.ReceiveDestroyed`
  (bind _returnvalue (`|SpawnActorFromClass` "/Game/Blueprint/Actors/BP_ACamera.BP_ACamera_C" (`SceneComponent.K2_GetComponentToWorld` (`self.Camera`)) "Undefined" "MultiplyWithRoot" null null)) ; adding a camera to maintain the momentum of death
  (`PlayerController.SetViewTargetWithBlend` (`GameplayStatics.GetPlayerController` 0) _returnvalue 0.0 "VTBlend_Linear" 0.0 false)
  (bind _asgm_tank_toon (cast `/Game/Blueprint/CORE/GM_TankToon` (`GameplayStatics.GetGameMode`)))
  (`/Game/Blueprint/CORE/GM_TankToon.PlayerDeath` _asgm_tank_toon))

(event `EnhancedInput|/Game/Blueprint/Inputs/Inputs/Shoot`
  (params (ActionValue :type Boolean) (ElapsedSeconds :type "Float (double-precision)") (TriggeredSeconds :type "Float (double-precision)") (InputAction :type "InputAction Object Reference" :default "/Game/Blueprint/Inputs/Inputs/Shoot.Shoot"))
  (:`Triggered`
    (`self.StartShoot` :!label _label))
  (:`Ongoing`
    (goto _label))
  (:`Completed`
    (`self.StopShoot`)))

(fn `SetMuzzle`
  (set `self.MuzzlePoint` (`self.TurretCannon`)))

(fn `UserConstructionScript`)