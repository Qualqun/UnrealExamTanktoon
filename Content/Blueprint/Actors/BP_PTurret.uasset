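; BP_PTurret is an enemy turret for the TankToon game mode that tracks and shoots the player within attack range.
; Each tick it checks distance to the player pawn, yaws the cannon toward it and calls StartShoot, otherwise StopShoot, while drawing a debug range sphere.
; It registers with GM_TankToon on BeginPlay and unregisters when destroyed, using the inherited shooting logic and muzzle point.
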(event `self.ReceiveBeginPlay`
  (`parent.ReceiveBeginPlay`)
  (set `self.MuzzlePoint` (`self.Muzzle`))
  (set `self.PlayerPawn` (`GameplayStatics.GetPlayerPawn` 0))
  (bind _asgm_tank_toon (cast `/Game/Blueprint/CORE/GM_TankToon` (`GameplayStatics.GetGameMode`)))
  (`/Game/Blueprint/CORE/GM_TankToon.SubscribeTurret` _asgm_tank_toon))

(event `self.ReceiveTick`
  (params (DeltaSeconds :type "Float (single-precision)"))
  (bind _returnvalue (`self.K2_GetActorLocation`))
  (bind _turretcannon (`self.TurretCannon`))
  (bind _returnvalue_2 (`self.K2_GetActorLocation` (`self.PlayerPawn`)))
  (bind (_returnvalue_roll _returnvalue_pitch _returnvalue_yaw) (`KismetMathLibrary.BreakRotator` (`KismetMathLibrary.FindLookAtRotation` (`SceneComponent.K2_GetComponentLocation` _turretcannon) _returnvalue_2)))
  (`KismetSystemLibrary.DrawDebugSphere` _returnvalue (`self.RangeAttack`) 12 (struct :`R` 1.0 :`G` 0.045875 :`A` 1.0))
  (`/Engine/EditorBlueprintResources/StandardMacros.IsValid` (`self.PlayerPawn`)
    (:`Is Valid`
      (if (< (`KismetMathLibrary.Vector_Distance` _returnvalue _returnvalue_2) (`self.RangeAttack`))
        (`SceneComponent.K2_SetWorldRotation` _turretcannon (`KismetMathLibrary.MakeRotator` 0.0 0.0 _returnvalue_yaw) false false)
        (`self.StartShoot`)
        (else
          (`self.StopShoot`))))))

(event `self.ReceiveDestroyed`
  (bind _asgm_tank_toon (cast `/Game/Blueprint/CORE/GM_TankToon` (`GameplayStatics.GetGameMode`)))
  (`/Game/Blueprint/CORE/GM_TankToon.UnsubscribeTurret` _asgm_tank_toon))

(fn `UserConstructionScript`)