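; Game mode for TankToon that runs the start countdown, win/lose messages and mouse crosshair.
; BeginPlay loops a delayed countdown on the main text widget, then enables player input, calls SetMuzzle on the tank and shows the crosshair, which Tick moves to the mouse.
; Turrets subscribe and unsubscribe to a counter that triggers the win message at zero.
; PlayerDeath shows the loss message and reloads the Main level after a delay.
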(event `self.ReceiveBeginPlay`
  (bind _returnvalue (`GameplayStatics.GetPlayerPawn` 0))
  (bind _returnvalue_2 (`|CreateWidget` "/Game/Blueprint/UI/WP_CrossHair.WP_CrossHair_C"))
  (set `self.CursorWidget` _returnvalue_2)
  (bind _returnvalue_3 (`|CreateWidget` "/Game/Blueprint/UI/WP_MainText.WP_MainText_C"))
  (bind _output_get (set `self.MainTextRef` _returnvalue_3))
  (`UserWidget.AddToViewport` _output_get 0)
  (`KismetSystemLibrary.Delay` (`self.DelayTexts`) :!label _label)
  (`/Game/Blueprint/UI/WP_MainText.Set Text` _output_get (`KismetTextLibrary.Conv_IntToText` (`self.SecondsStart`)))
  (bind _result (`/Engine/EditorBlueprintResources/StandardMacros.DecrementInt` (`self.SecondsStart`))
    (:`  `
      (if (> _result 0)
        (goto _label)
        (else
          (`KismetSystemLibrary.Delay` (`self.DelayTexts`))
          (`/Game/Blueprint/UI/WP_MainText.Set Text` _output_get "GO!")
          (`KismetSystemLibrary.Delay` (`self.DelayTexts`))
          (`self.EnableInput` _returnvalue (`GameplayStatics.GetPlayerController` 0))
          (bind _asbp_pmain_tank (cast `/Game/Blueprint/Actors/BP_PMainTank` _returnvalue))
          (`/Game/Blueprint/Actors/BP_PMainTank.SetMuzzle` _asbp_pmain_tank)
          (`/Game/Blueprint/UI/WP_MainText.Set Text` _output_get "")
          (`UserWidget.AddToViewport` (`self.CursorWidget`) 0))))))

(event `self.ReceiveTick`
  (params (DeltaSeconds :type "Float (single-precision)"))
  (bind _returnvalue (`WidgetLayoutLibrary.GetMousePositionOnViewport`))
  (`Widget.SetRenderTranslation` (`self.CursorWidget`) _returnvalue))

(event `SubscribeTurret`
  (`/Engine/EditorBlueprintResources/StandardMacros.IncrementInt` (`self.NbTurret`)))

(event `UnsubscribeTurret`
  (bind _result (`/Engine/EditorBlueprintResources/StandardMacros.DecrementInt` (`self.NbTurret`))
    (:`  `
      (if (<= _result 0)
        (`/Game/Blueprint/UI/WP_MainText.Set Text` (`self.MainTextRef`) "You WON!!")))))

(event `PlayerDeath`
  (`/Game/Blueprint/UI/WP_MainText.Set Text` (`self.MainTextRef`) "You lost!!!")
  (`KismetSystemLibrary.Delay` (`self.DelayRestart`))
  (`GameplayStatics.OpenLevelBySoftObjectPtr` "/Game/Maps/Main.Main"))

(fn `UserConstructionScript`)